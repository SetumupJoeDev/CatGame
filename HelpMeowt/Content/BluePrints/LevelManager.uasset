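; LevelManager advances the player through in-world levels, with an end cutscene after the last one.
; Its LoadNextLevel event increments CurrentLevel and moves the player character to the matching LevelStartPoints actor, then resets the character's values and increments the UI day index.
; Past the last start point, it plays the VetCutscene end scene through a character reference that is only assigned in the teleport branch.
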(event Custom|LoadNextLevel_Event
  (bind _returnvalue (Game|GetPlayerCharacter 0))
  (bind _currentlevel (Variables|Default|GetCurrentLevel))
  (bind _levelstartpoints (Variables|Default|GetLevelStartPoints))
  (Math|Integer|IncrementInt _currentlevel
    (:%20%20
      (if (>= _currentlevel (Utilities|Array|Length _levelstartpoints))
        (Default|PlayEndSceneEvent (Variables|/Game/FirstPersonBP/Blueprints/FirstPersonCharacter.FirstPersonCharacter_C|GetVetCutscene (stale _asfirst_person_character)))
        (else
          (Transformation|SetActorLocation _returnvalue (Transformation|GetActorLocation (Utilities|Array|Get(acopy) _levelstartpoints _currentlevel)) false false)
          (bind _asfirst_person_character (Utilities|Casting|CastToFirstPersonCharacter _returnvalue))
          (Default|ResetValuesEvent _asfirst_person_character)
          (Math|Integer|IncrementInt (Variables|/Game/BluePrints/Widgets/PlayerUI.PlayerUI_C|GetDayIndex (Variables|/Game/FirstPersonBP/Blueprints/FirstPersonCharacter.FirstPersonCharacter_C|GetPlayerUI _asfirst_person_character))))))))

(fn ConstructionScript)