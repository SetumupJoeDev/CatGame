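; Base cat that the player can feed treats and tame, with random fur and eye patterns applied through dynamic materials at BeginPlay.
; Treats play meows and change animation state; enough of them start purring, letting a taming attempt succeed instead of drawing a growl.
; Taming targets the last entry in the player's Followers and notifies CatAIController.
; FollowPlayer turns the mesh toward its target and lerps the actor closer beyond FollowDistance.
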(event EventBeginPlay
  (bind _mesh (Variables|Character|GetMesh))
  (bind _returnvalue (Rendering|Material|CreateDynamicMaterialInstance _mesh 0 "/Game/FirstPersonBP/MediumCatTextures/M_CatFur.M_CatFur" "None" :!class /Script/Engine.PrimitiveComponent))
  (Rendering|Material|SetScalarParameterValue _returnvalue "CatPattern" (.OutItem (Utilities|Array|Random (Variables|Default|GetCatPatterns))) :!class /Script/Engine.MaterialInstanceDynamic)
  (bind _returnvalue_2 (Rendering|Material|CreateDynamicMaterialInstance _mesh 1 "/Game/FirstPersonBP/MediumCatTextures/M_CatEyesFull.M_CatEyesFull" "None" :!class /Script/Engine.PrimitiveComponent))
  (Rendering|Material|SetScalarParameterValue _returnvalue_2 "EyePattern" (.OutItem (Utilities|Array|Random (Variables|Default|GetCatEyePatterns))) :!class /Script/Engine.MaterialInstanceDynamic))

(event EventTick
  (params (DeltaSeconds :type Float%20%28single-precision%29))
  (switch Utilities|FlowControl|Switch|SwitchonCatMood (Variables|Default|GetCurrentMood)))

(fn ConstructionScript
  (Variables|Default|SetFollowDistance 2e+02)
  (Variables|Default|SetFollowSpeed 0.75)
  (Variables|Default|SetCurrentMood "NewEnumerator1"))

(fn FollowPlayer
  (bind _returnvalue (Transformation|GetActorLocation))
  (bind _player (Variables|Default|GetPlayer))
  (bind _player_2 (Variables|Default|GetPlayer))
  (bind _returnvalue_2 (Transformation|GetActorLocation _player))
  (bind _returnvalue_3 (Transformation|GetActorLocation _player_2))
  (bind _returnvalue_4 (Math|Rotator|FindLookatRotation _returnvalue _returnvalue_2))
  ;[1 1 1] Rotates the cat to look at the player
  (Transformation|SetWorldRotation (Variables|Character|GetMesh) (Math|Rotator|MakeRotator (.roll _returnvalue_4) 0.0 (.yaw _returnvalue_4)) false false)
  ;[1 1 1] If the cat is further from the player than its follow distance, then it moves towards the player
  (if (> (Math|Vector|Distance(Vector) (Transformation|GetActorLocation) (Transformation|GetActorLocation (Variables|Default|GetPlayer))) (Variables|Default|GetFollowDistance))
    ;[1 1 1] Sets the cat's position using the newly calculated LERP vector
    (Transformation|SetActorLocation (Math|Vector|Lerp(Vector) (Transformation|GetActorLocation) (Math|Vector|MakeVector (.x _returnvalue_3) (.y _returnvalue_3) (.z (Transformation|GetActorLocation))) (* (Variables|Default|GetFollowSpeed) (Utilities|Time|GetWorldDeltaSeconds))) false false)))

(fn RecieveTreat
  (bind _purringsound (Variables|Default|GetPurringSound))
  (Math|Integer|IncrementInt (Variables|Default|GetNumTreatsGiven)
    (:%20%20
      (Audio|PlaySound2D (.OutItem (Utilities|Array|Random (Variables|Default|GetMeowSounds))) 1.0 1.0 0.0 0 0)
      (Variables|Default|SetAnimState "NewEnumerator2")
      (if (>= (Variables|Default|GetNumTreatsGiven) (Variables|Default|GetNumTreatsRequired))
        (if (not (Audio|Components|Audio|IsPlaying _purringsound))
          (if (Utilities|Enum|NotEqual(Enum) (Variables|Default|GetCurrentMood) "NewEnumerator0")
            (Variables|Default|SetAnimState "NewEnumerator3")
            (Audio|Components|Audio|Play _purringsound 0.0)))))))

(fn AttempttoTame
  (if (Utilities|Enum|Equal(Enum) (Variables|Default|GetCurrentMood) "NewEnumerator0")
    (return false)
    (elif (>= (Variables|Default|GetNumTreatsGiven) (Variables|Default|GetNumTreatsRequired))
      (Variables|Default|SetCurrentMood "NewEnumerator0")
      (Audio|Components|Audio|Stop (Variables|Default|GetPurringSound))
      (Audio|PlaySound2D "/Game/Sounds/CatSounds/Tamed.Tamed" 1.0 1.0 0.0 0 0)
      (Utilities|Casting|CastToCatAIController (AI|GetAIController self)
        (:then
          _)
        (:CastFailed
          _))
      (CallFunction|SetCatTamed)
      (return true)
      (else
        (Audio|PlaySound2D (.OutItem (Utilities|Array|Random (Variables|Default|GetGrowlSounds))) 1.0 1.0 0.0 0 0)
        (return false)))))

(fn SetCatTamed
  (bind _self self)
  (if (not (Utilities|IsValid (Variables|Default|GetPlayer)))
    (bind _asfirst_person_character (Utilities|Casting|CastToFirstPersonCharacter (Game|GetPlayerCharacter 0)))
    (Variables|Default|SetPlayer (Utilities|Array|Get(acopy) (Variables|/Game/FirstPersonBP/Blueprints/FirstPersonCharacter.FirstPersonCharacter_C|GetFollowers _asfirst_person_character) (- (Utilities|Array|Length (Variables|/Game/FirstPersonBP/Blueprints/FirstPersonCharacter.FirstPersonCharacter_C|GetFollowers _asfirst_person_character)) 1)))
    (Utilities|Casting|CastToCatAIController (AI|GetAIController _self))
    (bind _ascat_aicontroller (Utilities|Casting|CastToCatAIController (AI|GetAIController _self)))
    (Default|WasTamedEvent _ascat_aicontroller _asfirst_person_character)))