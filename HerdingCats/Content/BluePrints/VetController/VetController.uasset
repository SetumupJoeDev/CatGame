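; Vet controller Blueprint that steps a vet character through a timed sequence of behavior states.
; BeginPlay runs a one-shot chain of evenly spaced delays, triggering dance, wave, two talk variants and pet in turn.
; Each custom event only sets the CurrentState enum to its matching value.
; An idle event is also defined, but the sequence never calls it.
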(event Custom|VetPet_Event
  (Variables|Default|SetCurrentState "NewEnumerator5"))

(event Custom|VetWave_Event
  (Variables|Default|SetCurrentState "NewEnumerator1"))

(event Custom|VetTalk02_Event
  (Variables|Default|SetCurrentState "NewEnumerator3"))

(event Custom|VetTalk01_Event
  (Variables|Default|SetCurrentState "NewEnumerator2"))

(event Custom|VetIdle_Event
  (Variables|Default|SetCurrentState "NewEnumerator0"))

(event Custom|VetDance_Event
  (Variables|Default|SetCurrentState "NewEnumerator4"))

(event EventBeginPlay
  (Utilities|FlowControl|Delay 5.0)
  (CallFunction|VetDanceEvent)
  (Utilities|FlowControl|Delay 5.0)
  (CallFunction|VetWaveEvent)
  (Utilities|FlowControl|Delay 5.0)
  (CallFunction|VetTalk01Event)
  (Utilities|FlowControl|Delay 5.0)
  (CallFunction|VetTalk02Event)
  (Utilities|FlowControl|Delay 5.0)
  (CallFunction|VetPetEvent))

(fn ConstructionScript)